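; Player character Blueprint that handles basic keyboard movement and mouse look through Enhanced Input.
; On BeginPlay it adds the IA_Movement mapping context to the owning player controller's input subsystem.
; WASD input feeds AddMovementInput along the control rotation's forward and right vectors.
; Mouse input drives controller yaw and pitch, with the vertical axis negated.
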(event Input|EnhancedActionEvents|EnhancedInputActionIA_WASDMovement
  (params (ActionValue :type Vector%202D%20Structure) (ElapsedSeconds :type Float%20%28double-precision%29) (TriggeredSeconds :type Float%20%28double-precision%29) (InputAction :type Input%20Action%20Object%20Reference :default "/Game/IA_WASDMovement.IA_WASDMovement"))
  (bind _returnvalue (Pawn|GetControlRotation :!class /Script/Engine.Pawn))
  ;[0.15 0.15 0.15 0.5] Keyboard Movement
  ;;[0.15 0.15 0.15 0.5] Left/Right Movement
  (Pawn|Input|AddMovementInput (Math|Vector|GetRightVector _returnvalue) (.y ActionValue) false)
  ;;[0.15 0.15 0.15 0.5] Forward/Backward Movement
  (Pawn|Input|AddMovementInput (Math|Vector|GetForwardVector _returnvalue) (.x ActionValue) false))

(event Input|EnhancedActionEvents|EnhancedInputActionIA_MouseMovement
  (params (ActionValue :type Vector%202D%20Structure) (ElapsedSeconds :type Float%20%28double-precision%29) (TriggeredSeconds :type Float%20%28double-precision%29) (InputAction :type Input%20Action%20Object%20Reference :default "/Game/IA_MouseMovement.IA_MouseMovement"))
  ;[0.15 0.15 0.15 0.5] Mouse Looking Input
  (Pawn|Input|AddControllerYawInput (.x ActionValue))
  (Pawn|Input|AddControllerPitchInput (* (.y ActionValue) -1.0)))

(event EventBeginPlay
  ;[0.15 0.15 0.15 0.5] Init Character Controller
  (bind _asplayer_controller (Utilities|Casting|CastToPlayerController (Pawn|GetController)))
  (Input|AddMappingContext (PlayerController|LocalPlayerSubsystems|GetEnhancedInputLocalPlayerSubsystem _asplayer_controller) "/Game/IA_Movement.IA_Movement" 0 "(bIgnoreAllPressedKeysUntilRelease=True,bForceImmediately=False,bNotifyUserSettings=False)"))

(fn ConstructionScript)