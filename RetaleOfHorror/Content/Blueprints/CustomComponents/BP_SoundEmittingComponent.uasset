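; BP_SoundEmittingComponent is a component that starts and stops a given sound effect and tells hearing components about it.
; EmitAudio activates the sound without resetting it, while StopEmmittingAudio deactivates it.
; Both events then find every actor implementing BPI_ActorAudioCommunication and send a started or stopped message, with itself as source, to their BP_SoundHearingComponents.
; The broadcast applies no distance or filtering check.
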(event Custom|EmitAudio
  (params (SFXToPlay :type Audio%20Component%20Object%20Reference))
  ;[0.15 0.15 0.15 0.5] PlaySFX
  (Components|Activation|SetActive SFXToPlay true false)
  (bind _outactors (Actor|GetAllActorswithInterface "/Game/Blueprints/Interfaces/BPI_ActorAudioCommunication.BPI_ActorAudioCommunication_C"))
  (for _array_element _outactors
    (Class|BPIActorAudioCommunication|StartedAudio(Message) (Actor|GetComponentsByClass _array_element "/Game/Blueprints/CustomComponents/BP_SoundHearingComponent.BP_SoundHearingComponent_C") "This heard you" self)))

(event Custom|StopEmmittingAudio
  (params (SFX%20To%20pause :type Audio%20Component%20Object%20Reference))
  ;[0.15 0.15 0.15 0.5] PauseSFX
  (Components|Activation|Deactivate SFX%20To%20pause)
  (bind _outactors (Actor|GetAllActorswithInterface "/Game/Blueprints/Interfaces/BPI_ActorAudioCommunication.BPI_ActorAudioCommunication_C"))
  (for _array_element _outactors
    (Class|BPIActorAudioCommunication|StoppedAudio(Message) (Actor|GetComponentsByClass _array_element "/Game/Blueprints/CustomComponents/BP_SoundHearingComponent.BP_SoundHearingComponent_C") "It stopped hearing you" self)))